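; Player-controlled physics marble that rolls, jumps, respawns and can be teleported.
; Horizontal mouse movement applies torque to the sphere on X and Y, while vertical mouse input does nothing.
; Space replaces its velocity with a straight upward one, with no ground check.
; R returns it to its BeginPlay location at rest; Teleport moves it to a destination and rotates its linear velocity by that destination's rotation.
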(event EventBeginPlay
  ;[1 1 1] Remember starting location
  (Variables|Default|SetRespawn%20location (Transformation|GetWorldLocation (Variables|Default|GetSphere))))

(event Input|MouseEvents|MouseX
  (params (AxisValue :type Float%20%28single-precision%29))
  ;[1 1 1] Movement
  (Class|PrimitiveComponent|AddTorque (Variables|Default|GetSphere) (Math|Vector|MakeVector (* AxisValue 1e+06 -1.0) (* (stale Input|MouseEvents|MouseY AxisValue) 1e+06) 0.0) "None" false))

(event Input|MouseEvents|MouseY
  (params (AxisValue :type Float%20%28single-precision%29))
  ;[1 1 1] Movement
)

(event Input|KeyboardEvents|R
  (params (Key :type Key%20Structure :default "AnyKey"))
  (:Pressed
    (CallFunction|Respawn)))

(event Input|KeyboardEvents|SpaceBar
  (params (Key :type Key%20Structure :default "AnyKey"))
  (:Pressed
    (Physics|SetPhysicsLinearVelocity (Variables|Default|GetSphere) "0,0.000000,250.000000" false "None")))

(fn ConstructionScript)

(fn Respawn
  (Transformation|SetWorldLocation (Variables|Default|GetSphere) (Variables|Default|GetRespawn%20location) false false)
  (Physics|SetPhysicsLinearVelocity (Variables|Default|GetSphere) "0, 0, 0" false "None")
  (Class|PrimitiveComponent|SetPhysicsAngularVelocity (Variables|Default|GetSphere) "0, 0, 0" false "None"))

(fn Teleport
  (params (Destination :type Transform))
  (Transformation|SetWorldLocation (Variables|Default|GetSphere) (.location Destination) false false)
  (bind _returnvalue (Physics|GetPhysicsLinearVelocity (Variables|Default|GetSphere) "None"))
  (Physics|SetPhysicsLinearVelocity (Variables|Default|GetSphere) (Math|Vector|RotateVector _returnvalue (.rotation Destination)) false "None"))