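; SpinningFloor is an actor whose cylinder floor spins while something overlaps its sphere trigger.
; Overlap begin and end events set the IsRotating flag and start or stop the audio.
; Tick checks that flag and adds SpinSpeedAndDirection as local rotation each frame, without delta-time scaling.
; Overlaps are neither filtered nor counted, so any component leaving the trigger stops the spin.
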(event OnComponentBeginOverlap(SphereTrigger)
  (params (OtherActor :type Actor%20Object%20Reference) (OtherComp :type Primitive%20Component%20Object%20Reference) (OtherBodyIndex :type Integer) (bFromSweep :type Boolean) (SweepResult :type Hit%20Result%20Structure%20%28by%20ref%29))
  ;[1 1 1] Something triggered me. Record this state for the tick spinner
  (Audio|Components|Audio|Play (Variables|Default|GetAudio) 0.0)
  (Variables|Default|SetIsRotating true))

(event OnComponentEndOverlap(SphereTrigger)
  (params (OtherActor :type Actor%20Object%20Reference) (OtherComp :type Primitive%20Component%20Object%20Reference) (OtherBodyIndex :type Integer))
  ;[1 1 1] Something triggered me. Record this state for the tick spinner
  (Audio|Components|Audio|Stop (Variables|Default|GetAudio))
  (Variables|Default|SetIsRotating false))

(event EventTick
  (params (DeltaSeconds :type Float%20%28single-precision%29))
  ;[1 1 1] Make a decision based on our state
  (if (Variables|Default|GetIsRotating)
    ;[1 1 1] Actually rotate the floor
    (Transformation|AddLocalRotation (Variables|Default|GetCylinder) (Variables|Default|GetSpin%20speed%20and%20direction) false false)))

(fn ConstructionScript)