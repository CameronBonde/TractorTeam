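; Enemy marble that chases the player's MainMarble while it is nearby and heads back to its spawn point otherwise.
; A trigger sphere's overlap events store or clear the player's overlapping component as the target.
; Each tick, a physics force scaled by Speed pushes the sphere toward that target, or toward the home location saved at BeginPlay.
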(event OnComponentBeginOverlap(Spheretrigger)
  (params (OtherActor :type Actor%20Object%20Reference) (OtherComp :type Primitive%20Component%20Object%20Reference) (OtherBodyIndex :type Integer) (bFromSweep :type Boolean) (SweepResult :type Hit%20Result%20Structure%20%28by%20ref%29))
  ;[1 1 1] forget when the player moves outside the trigger
  (Utilities|Casting|CastToMainMarble OtherActor)
  (Variables|Default|SetMarble%20near%20me OtherComp))

(event OnComponentEndOverlap(Spheretrigger)
  (params (OtherActor :type Actor%20Object%20Reference) (OtherComp :type Primitive%20Component%20Object%20Reference) (OtherBodyIndex :type Integer))
  ;[1 1 1] check nearby marbles
  (Utilities|Casting|CastToMainMarble OtherActor)
  (Variables|Default|SetMarble%20near%20me 0))

(event EventBeginPlay
  ;[1 1 1] store location, so we can go back home
  (Variables|Default|SetHome%20location (Transformation|GetWorldLocation (Variables|Default|GetSphere))))

(event EventTick
  (params (DeltaSeconds :type Float%20%28single-precision%29))
  (if (Utilities|IsValid (Variables|Default|GetMarble%20near%20me))
    (Physics|AddForce (Variables|Default|GetSphere) (* (Class|KismetMathLibrary|GetDirectionVector (Transformation|GetWorldLocation (Variables|Default|GetSphere)) (Transformation|GetWorldLocation (Variables|Default|GetMarble%20near%20me))) (Variables|Default|Getspeed)) "None" false)
    (else
      (Physics|AddForce (Variables|Default|GetSphere) (* (Class|KismetMathLibrary|GetDirectionVector (Transformation|GetWorldLocation (Variables|Default|GetSphere)) (Variables|Default|GetHome%20location)) (Variables|Default|Getspeed)) "None" false))))

(fn ConstructionScript)