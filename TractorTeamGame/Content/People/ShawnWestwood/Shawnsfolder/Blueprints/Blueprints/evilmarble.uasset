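; Evil marble actor: a physics-driven sphere that chases whatever qualifying actor enters its trigger.
; SphereTrigger overlaps set the target to the entering component, or back to HomePoint when that actor leaves; the cast's class is not shown.
; Every tick, a constant-strength force pushes the sphere toward the target's current location.
; The start location saved in Home at BeginPlay is never read.
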(event OnComponentEndOverlap(Spheretrigger)
  (params (OtherActor :type Actor%20Object%20Reference) (OtherComp :type Primitive%20Component%20Object%20Reference) (OtherBodyIndex :type Integer))
  (Utilities|Casting|CastTo OtherActor)
  (Variables|Default|SetTarget%20component (Variables|Default|GetHome%20point)))

(event OnComponentBeginOverlap(Spheretrigger)
  (params (OtherActor :type Actor%20Object%20Reference) (OtherComp :type Primitive%20Component%20Object%20Reference) (OtherBodyIndex :type Integer) (bFromSweep :type Boolean) (SweepResult :type Hit%20Result%20Structure%20%28by%20ref%29))
  (Utilities|Casting|CastTo OtherActor)
  (Variables|Default|SetTarget%20component OtherComp))

(event EventBeginPlay
  (Variables|Components|SetHome (Transformation|GetWorldLocation (Variables|Default|GetSphere))))

(event EventTick
  (params (DeltaSeconds :type Float%20%28single-precision%29))
  (Physics|AddForce (Variables|Default|GetSphere) (* (Class|KismetMathLibrary|GetDirectionVector (Transformation|GetWorldLocation (Variables|Default|GetSphere)) (Transformation|GetWorldLocation (Variables|Default|GetTarget%20component))) 1e+05) "None" false))

(fn ConstructionScript)

(fn NewFunction0)