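; Sphere_Blueprint is a physics-driven sphere that the player rolls with the mouse, launches upward and can reset.
; Mouse X and Y both feed one AddTorque call that applies the same scaled value to the X and Y axes.
; Space overwrites the sphere's linear velocity with a fixed upward one, with no ground check.
; R calls Respawn, which restores the location saved at BeginPlay and zeroes linear and angular velocity.
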(event EventBeginPlay
  (Variables|Default|SetRespawn%20Location (Transformation|GetWorldLocation (Variables|Default|GetSphere))))

(event Input|MouseEvents|MouseX
  (params (AxisValue :type Float%20%28single-precision%29))
  (Class|PrimitiveComponent|AddTorque (Variables|Default|GetSphere) (Math|Vector|MakeVector (* AxisValue 1e+05) (* (stale Input|MouseEvents|MouseY AxisValue) 1e+05) 0.0) "None" false))

(event Input|MouseEvents|MouseY
  (params (AxisValue :type Float%20%28single-precision%29))
  (Class|PrimitiveComponent|AddTorque (Variables|Default|GetSphere) (Math|Vector|MakeVector (* (stale Input|MouseEvents|MouseX AxisValue) 1e+05) (* AxisValue 1e+05) 0.0) "None" false))

(event Input|KeyboardEvents|SpaceBar
  (params (Key :type Key%20Structure :default "AnyKey"))
  (:Pressed
    (Physics|SetPhysicsLinearVelocity (Variables|Default|GetSphere) "0, 0,250.000000" false "None")))

(event Input|KeyboardEvents|R
  (params (Key :type Key%20Structure :default "AnyKey"))
  (:Pressed
    (CallFunction|Respawn)))

(fn ConstructionScript)

(fn Respawn
  (Transformation|SetWorldLocation (Variables|Default|GetSphere) (Variables|Default|GetRespawn%20Location) false false)
  (Physics|SetPhysicsLinearVelocity (Variables|Default|GetSphere) "0, 0, 0" false "None")
  (Class|PrimitiveComponent|SetPhysicsAngularVelocity (Variables|Default|GetSphere) "0, 0, 0" false "None"))