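; A physics-driven sphere Blueprint that is rolled by horizontal mouse movement and can be reset to its start point.
; The MouseX axis applies opposing torque on X and Y to the Sphere component, while MouseY is left empty.
; BeginPlay saves the sphere's world location, and pressing R calls Respawn, which moves it back there and zeroes its linear and angular velocity.
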(event EventBeginPlay
  ;[1 1 1] Remember starting location
  (Variables|Default|SetRespwan%20loaction (Transformation|GetWorldLocation (Variables|Default|GetSphere))))

(event Input|MouseEvents|MouseX
  (params (AxisValue :type Float%20%28single-precision%29))
  ;[1 1 1] Movement
  (Class|PrimitiveComponent|AddTorque (Variables|Default|GetSphere) (Math|Vector|MakeVector (* AxisValue -1e+06) (* (stale Input|MouseEvents|MouseY AxisValue) 1e+06) 0.0) "None" false))

(event Input|MouseEvents|MouseY
  (params (AxisValue :type Float%20%28single-precision%29))
  ;[1 1 1] Movement
)

(event Input|KeyboardEvents|R
  (params (Key :type Key%20Structure :default "AnyKey"))
  (:Pressed
    (CallFunction|Respawn)))

(fn ConstructionScript)

(fn Respawn
  (Transformation|SetWorldLocation (Variables|Default|GetSphere) (Variables|Default|GetRespwan%20loaction) false false)
  (Physics|SetPhysicsLinearVelocity (Variables|Default|GetSphere) "0, 0, 0" false "None")
  (Class|PrimitiveComponent|SetPhysicsAngularVelocity (Variables|Default|GetSphere) "0, 0, 0" false "None"))