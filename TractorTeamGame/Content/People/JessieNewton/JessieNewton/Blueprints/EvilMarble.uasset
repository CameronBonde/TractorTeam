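; EvilMarble is an enemy physics marble that chases a nearby player marble (Sphere_Blueprint).
; Overlap events on its Collision component set and clear the chase target as marbles enter and leave.
; Each Tick it applies a fixed-strength force to its Sphere toward that target, without delta-time scaling.
; A Respawn function returns the Sphere to its BeginPlay location and zeroes linear and angular velocity.
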(event OnComponentBeginOverlap(Collision)
  (params (OtherActor :type Actor%20Object%20Reference) (OtherComp :type Primitive%20Component%20Object%20Reference) (OtherBodyIndex :type Integer) (bFromSweep :type Boolean) (SweepResult :type Hit%20Result%20Structure%20%28by%20ref%29))
  ;[1 1 1] Check nearby marble
  ;;[1 1 1] Check if the actor is a marble
  (bind _assphere_blueprint (Utilities|Casting|CastToSphere_Blueprint OtherActor))
  (Variables|Default|SetMarble%20Nearby _assphere_blueprint))

(event OnComponentEndOverlap(Collision)
  (params (OtherActor :type Actor%20Object%20Reference) (OtherComp :type Primitive%20Component%20Object%20Reference) (OtherBodyIndex :type Integer))
  ;[1 1 1] Forget when player moves outside the trigger
  (Utilities|Casting|CastToSphere_Blueprint OtherActor)
  (Variables|Default|SetMarble%20Nearby 0))

(event EventTick
  (params (DeltaSeconds :type Float%20%28single-precision%29))
  (if (Utilities|IsValid (Variables|Default|GetMarble%20Nearby))
    (Physics|AddForce (Variables|Default|GetSphere) (* (Class|KismetMathLibrary|GetDirectionVector (Transformation|GetWorldLocation (Variables|Default|GetSphere)) (Transformation|GetSocketLocation (Variables|/Game/JessieNewton/Blueprints/Sphere_Blueprint.Sphere_Blueprint_C|GetSphere (Variables|Default|GetMarble%20Nearby)) "None")) 1e+05) "None" false)))

(event EventBeginPlay
  (Variables|Default|SetHomeLocator (Transformation|GetWorldLocation (Variables|Default|GetSphere)))
  (Variables|Default|SetRespwan%20loaction (Transformation|GetWorldLocation (Variables|Default|GetSphere))))

(fn ConstructionScript)

(fn Respawn
  (Transformation|SetWorldLocation (Variables|Default|GetSphere) (Variables|Default|GetRespwan%20Loaction) false false)
  (Physics|SetPhysicsLinearVelocity (Variables|Default|GetSphere) "0, 0, 0" false "None")
  (Class|PrimitiveComponent|SetPhysicsAngularVelocity (Variables|Default|GetSphere) "0, 0, 0" false "None"))